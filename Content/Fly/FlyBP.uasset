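; Fly actor that wanders on the XZ plane and reacts to damage with a temporary animation.
; A looping timer, its interval randomized once at BeginPlay, picks random box targets.
; Tick interpolates Direction toward GetTargetDirection, whose direction node appears unconnected, then moves the fly with clamped pitch and updates debug components.
; SetTargetToMouseCursor offers cursor-based targeting but is not called here.
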(event Custom|NextTarget
  ;[1 1 1] Random target selection
  (Variables|Default|SetTargetLocation (Math|Random|RandomPointinBoundingBox (Math|Vector|MakeVector 0.0 (.Y (Math|Vector|BreakVector (Transformation|GetActorLocation))) -4e+01) (Math|Vector|MakeVector 6e+02 0.0 1e+02))))

(event EventAnyDamage
  (params (Damage :type Float%20%28single-precision%29) (DamageType :type Damage%20Type%20Object%20Reference) (InstigatedBy :type Controller%20Object%20Reference) (DamageCauser :type Actor%20Object%20Reference))
  ;[1 1 1] Taking Damage
  (Components|Animation|PlayAnimation "/Game/Fly/Fly_Anim_Skeleton_TakeDamage.Fly_Anim_Skeleton_TakeDamage" false)
  (Utilities|FlowControl|RetriggerableDelay 0.8)
  (Components|Animation|PlayAnimation "/Game/Fly/Fly_Anim_Skeleton_Idle.Fly_Anim_Skeleton_Idle" true))

(event EventBeginPlay
  ;[1 1 1] Random target selection
  (Utilities|Time|SetTimerbyEvent (delegate Custom|NextTarget) (Math|Random|RandomFloatinRange 2.0 5.0) true)
  (Variables|Default|SetTargetLocation (Math|Random|RandomPointinBoundingBox (Math|Vector|MakeVector 0.0 (.Y (Math|Vector|BreakVector (Transformation|GetActorLocation))) -4e+01) (Math|Vector|MakeVector 6e+02 0.0 1e+02))))

(event EventTick
  (params (DeltaSeconds :type Float%20%28single-precision%29))
  (bind _direction (Variables|Default|GetDirection))
  (bind _returnvalue (Math|Conversions|RotationFromXVector _direction))
  (bind (_pitch _yaw _roll) (Class|KismetMathLibrary|BreakRot _returnvalue))
  ;[1 1 1] Movement
  (bind _forwardvector (Utilities|CalcDirection DeltaSeconds)
    (:OUT
      (Transformation|SetActorLocationAndRotation (+ (* _forwardvector (* DeltaSeconds (Variables|Constants|GetSpeed))) (Transformation|GetActorLocation)) (Class|KismetMathLibrary|MakeRot (Math|Float|ClampAngle _pitch -2e+01 2e+01) _yaw _roll))
      ;[1 1 1] Debug components
      (Transformation|SetWorldRotation (Math|Conversions|RotationFromXVector (Variables|Default|GetDirection)) false)
      (Transformation|SetWorldLocation (Variables|Default|GetTargetLocation) false)
      (Transformation|SetWorldRotation (Math|Conversions|RotationFromXVector (Utilities|GetTargetDirection)) false))))

(fn ConstructionScript)