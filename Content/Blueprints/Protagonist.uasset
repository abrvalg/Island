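; Player character that moves side to side within a bounded area and throws rocks.
; The RightLeft axis adds movement input and flips the mesh to face the travel direction, while Tick clamps X and Z position.
; Jump input only toggles a Throwing flag; nothing here calls the Throw event.
; Throw spawns a Rock at the hand socket and launches it along the socket's forward vector.
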(event Custom|Throw
  (bind _returnvalue (Transformation|GetSocketTransform "hand" "RTS_World"))
  (bind _returnvalue_2 (Game|SpawnActorfromClass "/Game/Blueprints/Rock.Rock_C" _returnvalue true 0))
  (Physics|SetPhysicsLinearVelocity _returnvalue_2 (* (Math|Vector|RotateVector "1.000000, 0, 0" (.Rotation (Math|Transform|BreakTransform _returnvalue))) 8e+02) false "None"))

(event EventBeginPlay)

(event EventActorBeginOverlap
  (params (OtherActor :type Actor%20Object%20Reference)))

(event EventTick
  (params (DeltaSeconds :type Float%20%28single-precision%29))
  (bind _returnvalue (Transformation|GetWorldLocation))
  (bind (_x _y _z) (Math|Vector|BreakVector _returnvalue))
  (Transformation|SetWorldLocation (Math|Vector|MakeVector (Math|Float|Clamp(Float) _x -325.0 325.0) _y (Math|Float|Clamp(Float) _z -28.0 28.0)) false))

(event Input|ActionEvents|InputActionJump
  (:Pressed
    (Variables|Default|SetThrowing true))
  (:Released
    (Variables|Default|SetThrowing false)))

(event Input|AxisEvents|InputAxisRightLeft
  (params (AxisValue :type Float%20%28single-precision%29))
  (Class|PawnMovementComponent|AddInputVector (Math|Vector|MakeVector AxisValue 0.0 0.0) false)
  (Math|Float|CompareFloat AxisValue 0.0
    (:>
      (Transformation|SetWorldRotation (Variables|Character|GetMesh) "0,180.000000, 0" false))
    (:<
      (Transformation|SetWorldRotation (Variables|Character|GetMesh) "0, 0, 0" false))))

(fn ConstructionScript)