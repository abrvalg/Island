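; Destructible rock actor that breaks on its third physical hit.
; Each Hit event increments a counter and, up to the third, plays a rock sound at the impact point with volume scaled by impulse strength.
; On the third, Die attaches a destruction particle effect to the Box, destroys two components, hides visuals and removes the actor after a short delay.
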(event EventHit
  (params (MyComp :type Primitive%20Component%20Object%20Reference) (Other :type Actor%20Object%20Reference) (OtherComp :type Primitive%20Component%20Object%20Reference) (bSelfMoved :type Boolean) (HitLocation :type Vector :default "0, 0, 0") (HitNormal :type Vector :default "0, 0, 0") (NormalImpulse :type Vector :default "0, 0, 0") (Hit :type Hit%20Result%20Structure%20%28by%20ref%29))
  (bind _output_get (Variables|Default|SetHitCount (+ (Variables|Default|GetHitCount) 1)))
  (Math|Integer|CompareInt _output_get 3
    (:==
      (Utilities|FlowControl|Sequence
        (:then_0
          (Utilities|Die))
        (:then_1
          (Audio|PlaySoundatLocation "/Game/Sound/rock.rock" HitLocation (/ (Math|Vector|VectorLength NormalImpulse) 5e+02) :!label _label))))
    (:<
      (goto _label))))

(event EventBeginPlay)

(event EventActorBeginOverlap
  (params (OtherActor :type Actor%20Object%20Reference)))

(event EventTick
  (params (DeltaSeconds :type Float%20%28single-precision%29)))

(fn ConstructionScript)