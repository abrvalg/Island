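; Spawner actor that keeps adding FlyBP actors to the level up to a MaxCount limit.
; A looping timer started on BeginPlay counts all FlyBP actors in the world and spawns one while the count is below the limit.
; Spawn transforms come from RandomTransform, whose random-point-in-Box transform node is present but unconnected in that graph.
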(event Custom|TrySpawn
  (bind _outactors (Actor|GetAllActorsOfClass "/Game/Enemy/FlyBP.FlyBP_C"))
  (Math|Integer|CompareInt (Utilities|Array|Length _outactors) (Variables|Default|GetMaxCount)
    (:<
      (Game|SpawnActorfromClass "/Game/Enemy/FlyBP.FlyBP_C" (Utilities|RandomTransform) false 0))))

(event EventBeginPlay
  (Utilities|Time|SetTimerbyEvent (delegate Custom|TrySpawn) 3.0 true))

(event EventActorBeginOverlap
  (params (OtherActor :type Actor%20Object%20Reference)))

(event EventTick
  (params (DeltaSeconds :type Float%20%28single-precision%29)))

(fn ConstructionScript)